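; Player-controllable tank pawn Blueprint that wires components to native tank logic and routes input.
; On BeginPlay it registers the barrel and turret and initializes the movement component with both tracks.
; Aim axes rotate an azimuth gimbal and spring arm for the camera.
; Movement input drives each track's throttle directly or passes forward and turn intent to the movement component, and the fire action calls Fire.
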(event `self.ReceiveBeginPlay`
  (`self.SetBarrelReference` (`self.TankBarrel`))
  (`self.SetTurretReference` (`self.TankTurret`))
  (`TankMovementComponent.Initialize` (`self.TankMovement`) (`self.TankTrackL`) (`self.TankTrackR`)))

(event `InputAxis|AimAzimuth`
  (params (AxisValue :type "Float (single-precision)"))
  ;[1 1 1] Camera input bindings
  (`SceneComponent.K2_AddLocalRotation` (`self.Azimuth Gimbal`) (`KismetMathLibrary.MakeRotator` 0.0 0.0 AxisValue) false false))

(event `InputAxis|Left track throttle`
  (params (AxisValue :type "Float (single-precision)"))
  ;[1 1 1] Movement input bindings
  (`TankTrack.SetThrottle` (`self.TankTrackL`) AxisValue))

(event `InputAxis|Right track throttle`
  (params (AxisValue :type "Float (single-precision)"))
  ;[1 1 1] Movement input bindings
  (`TankTrack.SetThrottle` (`self.TankTrackR`) AxisValue))

(event `InputAxis|AimElevation`
  (params (AxisValue :type "Float (single-precision)"))
  ;[1 1 1] Camera input bindings
  (`SceneComponent.K2_AddLocalRotation` (`self.SpringArm`) (`KismetMathLibrary.MakeRotator` 0.0 AxisValue) false false))

(event `InputAxis|Forward backward`
  (params (AxisValue :type "Float (single-precision)"))
  ;[1 1 1] Movement input bindings
  (`TankMovementComponent.IntendMoveFoward` (`self.TankMovement`) AxisValue))

(event `InputAxis|Turn Right`
  (params (AxisValue :type "Float (single-precision)"))
  ;[1 1 1] Movement input bindings
  (`TankMovementComponent.IntendTurnRight` (`self.TankMovement`) AxisValue))

(event `InputAction|Fire`
  (params (Key :type "Key Structure"))
  (:`Pressed`
    (`self.Fire`)))

(fn `UserConstructionScript`)